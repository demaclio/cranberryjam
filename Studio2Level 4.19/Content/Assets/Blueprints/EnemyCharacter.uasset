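; Enemy character that takes damage, shows a health bar and notifies the dream meter and spawner when killed.
; BeginPlay binds the health bar widget and finds the DreamMeter and EnemySpawner.
; AnyDamage lowers health, spawns damage text or destroys the enemy at zero, and starts a looping FollowCharacter timer that turns the bar toward the damage causer.
; Contact damage and body colour logic are left unconnected.
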(event OnComponentBeginOverlap(Box)
  (params (OverlappedComponent :type Primitive%20Component%20Object%20Reference) (OtherActor :type Actor%20Object%20Reference) (OtherComp :type Primitive%20Component%20Object%20Reference) (OtherBodyIndex :type Integer) (bFromSweep :type Boolean) (SweepResult :type Hit%20Result%20Structure%20%28by%20ref%29))
  ;[1 1 1] Enemy Damage ----> Player
)

(event EventBeginPlay
  ;[1 1 1] Update Enemy Healthbar with Damage
  (bind _asenemy_health_bar (Utilities|Casting|CastToEnemyHealthBar (UserInterface|GetUserWidgetObject (Variables|Default|GetHealthBar))))
  (Variables|/Game/Assets/UI/EnemyHealthBar.EnemyHealthBar_C|SetOwner _asenemy_health_bar self)
  (bind _foundwidgets (Widget|GetAllWidgetsOfClass "/Game/Assets/UI/DreamMeter.DreamMeter_C" true))
  (Variables|Default|SetDreamWidget (Utilities|Array|Get(acopy) _foundwidgets))
  (bind _outactors (Actor|GetAllActorsOfClass "/Game/Assets/Blueprints/EnemySpawner.EnemySpawner_C"))
  (Variables|Default|SetEnemySpawner (Utilities|Array|Get(acopy) _outactors)))

(event Collision|EventActorBeginOverlap
  (params (OtherActor :type Actor%20Object%20Reference)))

(event EventTick
  (params (DeltaSeconds :type Float%20%28single-precision%29)))

(event Game|Damage|EventAnyDamage
  (params (Damage :type Float%20%28single-precision%29) (DamageType :type Damage%20Type%20Object%20Reference) (InstigatedBy :type Controller%20Object%20Reference) (DamageCauser :type Actor%20Object%20Reference))
  (bind _self self)
  (bind _returnvalue (Transformation|GetActorLocation _self))
  ;[1 1 1] Player Damages The Enemy
  (Variables|Default|SetAICurrentHealth (- (Variables|Default|GetAICurrentHealth) Damage))
  (Variables|Default|SetEnemy DamageCauser)
  (Rendering|SetVisibility (Variables|Default|GetHealthBar) true false)
  (bind _returnvalue_2 (Utilities|Time|SetTimerbyFunctionName 0 "FollowCharacter" 0.01 true))
  (Variables|Default|SetFollowCharacterhandle _returnvalue_2)
  (if (<= (Variables|Default|GetAICurrentHealth) 0.0)
    (Actor|DestroyActor)
    (Audio|PlaySoundatLocation "/Game/Assets/Audio/enemy/DeathSound01.DeathSound01" _returnvalue "0, 0, 0" 3.0)
    (Utilities|Casting|CastToDreamMeterClass "/Game/Assets/UI/DreamMeter.DreamMeter_C")
    (Default|EnemyRepelled (Variables|Default|GetDreamWidget))
    (Utilities|Casting|CastToEnemySpawnerClass "/Game/Assets/Blueprints/EnemySpawner.EnemySpawner_C")
    (Default|SpawnMonsters (Variables|Default|GetEnemySpawner))
    (else
      (Audio|PlaySoundatLocation "/Game/Assets/Audio/enemy/Sizzling2_0.Sizzling2_0" _returnvalue)
      (Game|SpawnActorfromClass "/Game/Assets/UI/DamageText.DamageText_C" (Math|Transform|MakeTransform (.location (Transformation|GetWorldTransform (Variables|Default|GetDamageText))) "0, 0, 0" "1,1,1") "Undefined" 0 (Variables|Default|GetEnemy) Damage 0))))

(fn ConstructionScript
  ;[1 1 1] Enemy Colour
)

(fn FollowCharacter
  (bind _returnvalue (Transformation|GetActorLocation))
  (bind _enemy (Variables|Default|GetEnemy))
  (bind _returnvalue_2 (Transformation|GetActorLocation _enemy))
  (bind _returnvalue_3 (Math|Rotator|FindLookatRotation _returnvalue _returnvalue_2))
  (Utilities|Casting|CastToEnemy_waypoint (Variables|Default|GetEnemy))
  (Transformation|SetWorldRotation (Variables|Default|GetHealthBar) (Math|Rotator|MakeRotator (.roll (Transformation|GetWorldRotation (Variables|Default|GetHealthBar))) (.pitch _returnvalue_3) (.yaw _returnvalue_3)) false false))