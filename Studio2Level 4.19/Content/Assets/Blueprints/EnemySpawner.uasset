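; Enemy spawner actor that spawns EnemyCharacter AI at random points inside its SpawnVolume box across two kill-driven waves.
; SpawnWave starts at BeginPlay and picks wave one or two by whether EnemiesKilled lies between the two wave limits.
; It spawns while live and total spawned counts stay below that wave's limit, re-calling itself after a short delay.
; SpawnMonsters counts a kill and re-runs the wave check.
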(event Custom|Spawn%20Wave
  (bind _spawnvolume (Variables|Default|GetSpawnVolume))
  ;[1 1 1] Enemy Spawning
  (if (Math|Integer|InRange(Integer) (Variables|Default|GetEnemiesKilled) (Variables|Default|GetWave%201%20Max) (Variables|Default|GetWave%202%20Max))
    (Variables|Default|SetWave%202 true)
    (Development|PrintString "Wave 2 Spawn")
    (bind _outactors (Actor|GetAllActorsOfClass "/Game/Assets/Blueprints/EnemyCharacter.EnemyCharacter_C"))
    (if (< (Utilities|Array|Length _outactors) (Variables|Default|GetWave%202%20Max))
      (if (< (Variables|Default|GetEnemiesSpawned) (Variables|Default|GetWave%202%20Max))
        (AI|SpawnAIFromClass "/Game/Assets/Blueprints/EnemyCharacter.EnemyCharacter_C" 0 (Math|Random|RandomPointinBoundingBox (Transformation|GetWorldLocation _spawnvolume) (Components|Box|GetScaledBoxExtent _spawnvolume)) "0, 0, 0" false :!label _label)
        (Variables|Default|SetEnemiesSpawned (+ (Variables|Default|GetEnemiesSpawned) 1))
        (if (Variables|Default|GetWave1)
          (Utilities|FlowControl|Delay 2.0)
          (CallFunction|SpawnWave :!label _label_2)
          (elif (Variables|Default|GetWave%202)
            (Utilities|FlowControl|Delay 2.0)
            (goto _label_2)))))
    (else
      (Variables|Default|SetWave1 true)
      (Development|PrintString "Wave 1 Spawn")
      (bind _outactors_2 (Actor|GetAllActorsOfClass "/Game/Assets/Blueprints/EnemyCharacter.EnemyCharacter_C"))
      (if (Variables|Default|GetWave1)
        (if (< (Utilities|Array|Length _outactors_2) (Variables|Default|GetWave%201%20Max))
          (if (< (Variables|Default|GetEnemiesSpawned) (Variables|Default|GetWave%201%20Max))
            (goto _label)))))))

(event Custom|SpawnMonsters
  (bind _spawnvolume (Variables|Default|GetSpawnVolume))
  ;[1 1 1] Enemy Spawning
  (Variables|Default|SetEnemiesKilled (+ (Variables|Default|GetEnemiesKilled) 1))
  (if (Math|Integer|InRange(Integer) (Variables|Default|GetEnemiesKilled) (Variables|Default|GetWave%201%20Max) (Variables|Default|GetWave%202%20Max))
    (Variables|Default|SetWave%202 true)
    (Development|PrintString "Wave 2 Spawn")
    (bind _outactors (Actor|GetAllActorsOfClass "/Game/Assets/Blueprints/EnemyCharacter.EnemyCharacter_C"))
    (if (< (Utilities|Array|Length _outactors) (Variables|Default|GetWave%202%20Max))
      (if (< (Variables|Default|GetEnemiesSpawned) (Variables|Default|GetWave%202%20Max))
        (AI|SpawnAIFromClass "/Game/Assets/Blueprints/EnemyCharacter.EnemyCharacter_C" 0 (Math|Random|RandomPointinBoundingBox (Transformation|GetWorldLocation _spawnvolume) (Components|Box|GetScaledBoxExtent _spawnvolume)) "0, 0, 0" false :!label _label)
        (Variables|Default|SetEnemiesSpawned (+ (Variables|Default|GetEnemiesSpawned) 1))
        (if (Variables|Default|GetWave1)
          (Utilities|FlowControl|Delay 2.0)
          (CallFunction|SpawnWave :!label _label_2)
          (elif (Variables|Default|GetWave%202)
            (Utilities|FlowControl|Delay 2.0)
            (goto _label_2)))))
    (else
      (Variables|Default|SetWave1 true)
      (Development|PrintString "Wave 1 Spawn")
      (bind _outactors_2 (Actor|GetAllActorsOfClass "/Game/Assets/Blueprints/EnemyCharacter.EnemyCharacter_C"))
      (if (Variables|Default|GetWave1)
        (if (< (Utilities|Array|Length _outactors_2) (Variables|Default|GetWave%201%20Max))
          (if (< (Variables|Default|GetEnemiesSpawned) (Variables|Default|GetWave%201%20Max))
            (goto _label)))))))

(event EventBeginPlay
  (CallFunction|SpawnWave))

(event Collision|EventActorBeginOverlap
  (params (OtherActor :type Actor%20Object%20Reference)))

(event EventTick
  (params (DeltaSeconds :type Float%20%28single-precision%29)))

(fn ConstructionScript)